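; Paper2D side-scrolling player character with Enhanced Input movement, jumping and a sword attack.
; Tick turns the controller to face travel, picks idle or run flipbooks outside attacks, and syncs footstep sounds to run frames.
; Specific attack frames trigger a DoOnce-gated hitbox check that damages Boss actors.
; Incoming damage lowers health, swaps to hit or death flipbooks, and shows the GameOver widget at zero.
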(event OnFinishedPlaying(Sprite)
  (bind _sprite (Variables|Default|GetSprite))
  (Variables|Default|SetIsAttacking false)
  (if (not (Variables|Default|GetIsDead))
    (Components|Timeline|SetLooping _sprite true)
    (Audio|Components|Audio|Play _sprite)
    (Development|SetHiddeninGame (Variables|Default|GetHitBox) true false)))

(event Custom|SetCharRotation
  (Math|Float|CompareFloat (.x (Variables|/Script/Engine.MovementComponent|GetVelocity (Variables|Character|GetCharacterMovement))) 0.0
    (:>
      ;[0 0.4745 1] Look Right
      (bind _asplayer_controller (Utilities|Casting|CastToPlayerController (Pawn|GetController)))
      (Pawn|SetControlRotation _asplayer_controller (Math|Rotator|MakeRotator 0.0 0.0 0.0)))
    (:<
      ;[0 0.4745 1] Look Left
      (bind _asplayer_controller_2 (Utilities|Casting|CastToPlayerController (Pawn|GetController)))
      (Pawn|SetControlRotation _asplayer_controller_2 (Math|Rotator|MakeRotator 0.0 0.0 1.8e+02)))))

(event Custom|Foot%20Sound
  (bind _sprite (Variables|Default|GetSprite))
  (bind _returnvalue (Class|PaperFlipbookComponent|GetPlaybackPositioninFrames _sprite))
  (if (== (Class|PaperFlipbookComponent|GetFlipbook (Variables|Default|GetSprite)) "/Game/Main_Character/Flipbook/Run_Flipbook.Run_Flipbook")
    (if (or (== _returnvalue 0) (== _returnvalue 2))
      (Utilities|FlowControl|DoOnce false :!label _label
        (:Completed
          (Audio|PlaySoundatLocation "/Game/Assets/Audio/running_Cue.running_Cue" (Transformation|GetActorLocation) "0, 0, 0" 1.0 1.0 0.0 0 0 0 0)))
      (else
        (goto _label Reset)))))

(event Custom|Check_Hitbox
  (bind _sprite (Variables|Default|GetSprite))
  (bind _returnvalue (Class|PaperFlipbookComponent|GetPlaybackPositioninFrames _sprite))
  (if (== (Class|PaperFlipbookComponent|GetFlipbook (Variables|Default|GetSprite)) "/Game/Main_Character/Flipbook/Attack_Flipbook.Attack_Flipbook")
    (if (or (== _returnvalue 4) (== _returnvalue 5))
      (for _array_element (Collision|GetOverlappingActors (Variables|Default|GetHitBox) "/Script/Engine.Actor" :!class /Script/Engine.PrimitiveComponent)
        (if (!= _array_element self)
          (Actor|DestroyActor _array_element))))))

(event Custom|Reset_Attack
  (Utilities|FlowControl|DoOnce false) ; enters at Reset
)

(event Input|EnhancedActionEvents|EnhancedInputActionIA_movement
  (params (ActionValue :type Float%20%28double-precision%29) (ElapsedSeconds :type Float%20%28double-precision%29) (TriggeredSeconds :type Float%20%28double-precision%29) (InputAction :type Input%20Action%20Object%20Reference :default "/Game/Main_Character/Input/Actions/IA_movement.IA_movement"))
  (:Triggered
    (Pawn|Input|AddMovementInput "1.000000,0.000000,0.000000" ActionValue false)))

(event Input|EnhancedActionEvents|EnhancedInputActionIA_Attack_1
  (params (ActionValue :type Boolean) (ElapsedSeconds :type Float%20%28double-precision%29) (TriggeredSeconds :type Float%20%28double-precision%29) (InputAction :type Input%20Action%20Object%20Reference :default "/Game/Main_Character/Input/Actions/IA_Attack_1.IA_Attack_1"))
  (bind _sprite (Variables|Default|GetSprite))
  (:Started
    (Variables|Default|SetIsAttacking true)
    (CallFunction|ResetAttack)
    (Components|Timeline|SetLooping _sprite false)
    (Sprite|SetFlipbook _sprite "/Game/Main_Character/Flipbook/Attack_Flipbook.Attack_Flipbook")
    (Audio|PlaySound2D "/Game/Assets/Audio/Sword_miss_Cue.Sword_miss_Cue" 1.0 1.0 0.0 0 0)))

(event EventBeginPlay
  (bind _asplayer_controller (Utilities|Casting|CastToPlayerController (Game|GetPlayerController 0)))
  (Input|AddMappingContext (PlayerController|LocalPlayerSubsystems|GetEnhancedInputLocalPlayerSubsystem _asplayer_controller) "/Game/Main_Character/Input/Actions/IMC_Main.IMC_Main" 0 "(bIgnoreAllPressedKeysUntilRelease=True,bForceImmediately=False)"))

(event EventTick
  (params (DeltaSeconds :type Float%20%28single-precision%29))
  (bind _sprite (Variables|Default|GetSprite))
  (bind _returnvalue (Class|PaperFlipbookComponent|GetPlaybackPositioninFrames _sprite))
  (CallFunction|SetCharRotation)
  (CallFunction|UpdateSprite)
  (CallFunction|FootSound)
  (if (Variables|Default|GetIsAttacking)
    (if (or (== _returnvalue 4) (== _returnvalue 5))
      (Utilities|FlowControl|DoOnce false
        (:Completed
          (CallFunction|HitCheck)
          (Development|SetHiddeninGame (Variables|Default|GetHitBox) false false)))
      (else
        (Development|SetHiddeninGame (Variables|Default|GetHitBox) true false)))))

(event Game|Damage|EventAnyDamage
  (params (Damage :type Float%20%28single-precision%29) (DamageType :type Damage%20Type%20Object%20Reference) (InstigatedBy :type Controller%20Object%20Reference) (DamageCauser :type Actor%20Object%20Reference))
  (bind _sprite (Variables|Default|GetSprite))
  (bind _sprite_2 (Variables|Default|GetSprite))
  (Variables|Default|SetHealth (- (Variables|Default|GetHealth) Damage))
  (if (<= (Variables|Default|GetHealth) 0.0)
    (bind _returnvalue (UserInterface|CreateWidget "/Game/UI/GameOver.GameOver_C"))
    (UserInterface|Viewport|AddtoViewport _returnvalue 0)
    (Sprite|SetFlipbook _sprite "/Game/Main_Character/Flipbook/Death_Flipbook.Death_Flipbook")
    (Components|Timeline|SetLooping _sprite_2 false)
    (Variables|Default|SetIsDead true)
    (else
      (Sprite|SetFlipbook _sprite "/Game/Main_Character/Flipbook/Hit_Flipbook.Hit_Flipbook")
      (Components|Timeline|SetLooping _sprite_2 true))))

(event Input|ActionEvents|InputActionJumping
  (params (Key :type Key%20Structure :default "None"))
  (bind _sprite (Variables|Default|GetSprite))
  (:Pressed
    (Variables|Default|SetIsJumping (Variables|Default|GetIsJumping))
    (Character|Jump)
    (Components|Timeline|SetLooping (Variables|Default|GetSprite) false)
    (Sprite|SetFlipbook _sprite "/Game/Main_Character/Flipbook/Jump_Flipbook.Jump_Flipbook")
    (Utilities|FlowControl|Delay 0.1)
    (if (== (.Z (Math|Vector|BreakVector (Transformation|GetVelocity))) 0.0) :!label _label
      (Components|Timeline|SetLooping _sprite true)
      (Audio|Components|Audio|Play _sprite)
      (Sprite|SetFlipbook _sprite "/Game/Main_Character/Flipbook/Idle_Flipbook.Idle_Flipbook")
      (Variables|Default|SetIsJumping false)
      (else
        (Utilities|FlowControl|Delay 0.1)
        (goto _label)))))

(fn ConstructionScript)

(fn UpdateSprite
  (if (not (Variables|Default|GetIsAttacking))
    (if (<= (Math|Float|Absolute(Float) (Math|Vector|VectorLength (Transformation|GetVelocity))) 0.0)
      (Sprite|SetFlipbook (Variables|Default|GetSprite) "/Game/Main_Character/Flipbook/Idle_Flipbook.Idle_Flipbook")
      (else
        (Sprite|SetFlipbook (Variables|Default|GetSprite) "/Game/Main_Character/Flipbook/Run_Flipbook.Run_Flipbook")))))

(fn HitCheck
  (for _array_element (Collision|GetOverlappingActors (Variables|Default|GetHitBox) "/Game/Enemies/NightBorne/Blueprint/Boss.Boss_C" :!class /Script/Engine.PrimitiveComponent)
    (if (!= _array_element self)
      (Game|Damage|ApplyDamage _array_element (Variables|Default|GetDamage%20Amount) 0 0)
      (Variables|Default|SetHitSomething true)))
  (if (Variables|Default|GetHitSomething)
    (Effects|SpawnEmitteratLocation 0 "0, 0, 0")
    (Audio|PlaySound2D "/Game/Assets/Audio/Sword_hit_Cue.Sword_hit_Cue" 1.0 1.0 0.0 0 0)))