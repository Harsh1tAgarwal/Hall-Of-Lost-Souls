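; Skeleton enemy Blueprint that damages overlapping Side_Character actors and takes damage itself.
; Tick watches its HitBox and, on sprite frame 4 or 8, runs HitCheck through a DoOnce gate re-armed by the ResetAttack event.
; HitCheck sets the attack flipbook and applies damage.
; Incoming damage reduces health and plays a hit flipbook, or sets the death flipbook and destroys the actor immediately at zero or below.
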(event Custom|ResetAttack
  (Utilities|FlowControl|DoOnce false) ; enters at Reset
)

(event EventTick
  (params (DeltaSeconds :type Float%20%28single-precision%29))
  (bind _sprite (Variables|Default|GetSprite))
  (bind _returnvalue (Class|PaperFlipbookComponent|GetPlaybackPositioninFrames _sprite))
  (for _array_element (Collision|GetOverlappingActors (Variables|Default|GetHitBox) "/Game/Main_Character/Blueprints/Side_Character.Side_Character_C" :!class /Script/Engine.PrimitiveComponent)
    (if (or (== _returnvalue 4) (== _returnvalue 8))
      (Utilities|FlowControl|DoOnce false
        (:Completed
          (CallFunction|HitCheck))))))

(event Game|Damage|EventAnyDamage
  (params (Damage :type Float%20%28single-precision%29) (DamageType :type Damage%20Type%20Object%20Reference) (InstigatedBy :type Controller%20Object%20Reference) (DamageCauser :type Actor%20Object%20Reference))
  (bind _sprite (Variables|Default|GetSprite))
  (bind _sprite_2 (Variables|Default|GetSprite))
  (Variables|Default|SetHealth (- (Variables|Default|GetHealth) Damage))
  (if (<= (Variables|Default|GetHealth) 0.0)
    (Sprite|SetFlipbook _sprite "/Game/Enemies/Skeleton_enemy/Skeleton_enemy/Flipbook/Skel_Death.Skel_Death")
    (Components|Timeline|SetLooping _sprite false)
    (Actor|DestroyActor)
    (else
      (Sprite|SetFlipbook _sprite_2 "/Game/Enemies/Skeleton_enemy/Skeleton_enemy/Flipbook/Skel_hit.Skel_hit")
      (Components|Timeline|SetLooping _sprite_2 false))))

(fn ConstructionScript)

(fn HitCheck
  (for _array_element (Collision|GetOverlappingActors (Variables|Default|GetHitBox) "/Game/Main_Character/Blueprints/Side_Character.Side_Character_C" :!class /Script/Engine.PrimitiveComponent)
    (if (!= _array_element self)
      (Sprite|SetFlipbook (Variables|Default|GetSprite) "/Game/Enemies/Skeleton_enemy/Skeleton_enemy/Flipbook/Skel_attack.Skel_attack")
      (Game|Damage|ApplyDamage _array_element (Variables|Default|GetDamageAmount) 0 0))))